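; BaseSword is a sword weapon Blueprint that deals melee damage to nearby pawns.
; Its TryDealDamage event runs a WeaponRange sphere overlap at the SwordMesh location and applies WeaponDamage to every pawn found.
; It excludes the wielder by resolving the owner of the root component's attach parent.
; The event is not triggered within this Blueprint, and BeginPlay, overlap, Tick and the construction script are empty.
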(event `TryDealDamage`
  (bind _outactors (`KismetSystemLibrary.SphereOverlapActors` (`SceneComponent.K2_GetComponentLocation` (`self.SwordMesh`)) (`self.WeaponRange`) (`|MakeArray` "ObjectTypeQuery3" :!type "EObjectTypeQuery Enum") null (`|MakeArray` (`ActorComponent.GetOwner` (`SceneComponent.GetAttachParent` (`self.DefaultSceneRoot`))))))
  (for _array_element _outactors
    (`GameplayStatics.ApplyDamage` _array_element (`self.WeaponDamage`))))

(fn `UserConstructionScript`)