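; Game mode for a wave-based knight game that spawns AI enemies and the player's chosen pawn.
; Each wave's class list is shuffled into a queue, which a looping timer drains at random PlayerStarts.
; Enemy destruction starts the next wave once queue and AI controllers are empty; after the last, it blends to a random camera and opens MainMenu.
; The player pawn class comes from KnightGameInstance and spawns at a ControledPlayerStart.
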(event `self.ReceiveBeginPlay`
  (`KismetSystemLibrary.K2_SetTimerDelegate` (delegate `SpawnEnemy`) 2.0 true)
  (`self.ResetGame`))

(event `SpawnEnemy`
  ;[1 1 1] Spawning AI enemy in random place (where is player spawner)
  (if (> (`KismetArrayLibrary.Array_Length` (`self.Queue`)) 0)
    (bind _outactors (`GameplayStatics.GetAllActorsOfClass` "/Script/Engine.PlayerStart"))
    (bind _output (`|GetArrayItem` _outactors (`KismetMathLibrary.RandomInteger` (`KismetArrayLibrary.Array_Length` _outactors))))
    (bind _returnvalue (`AIBlueprintHelperLibrary.SpawnAIFromClass` (`|GetArrayItem` (`self.Queue`)) null (`self.K2_GetActorLocation` _output) (`self.K2_GetActorRotation` _output)))
    (`KismetArrayLibrary.Array_Remove` (`self.Queue`))
    (bind _outactors_2 (`GameplayStatics.GetAllActorsOfClass` "/Game/Blueprints/KGAIControlerBase.KGAIControlerBase_C"))
    (set `self.EnemiesNum` (`KismetArrayLibrary.Array_Length` _outactors_2))
    (add `self.OnDestroyed` _returnvalue (delegate `CheckWaveCompleted`))))

(event `CheckWaveCompleted` :!signature `self.OnDestroyed`
  (params (DestroyedActor :type "Actor Object Reference"))
  (if (== (`KismetArrayLibrary.Array_Length` (`self.Queue`)) 0)
    ;[1 1 1] There is any enemies on the map?
    (bind _outactors (`GameplayStatics.GetAllActorsOfClass` "/Game/Blueprints/KGAIControlerBase.KGAIControlerBase_C"))
    (bind _returnvalue (`KismetArrayLibrary.Array_Length` _outactors))
    (set `self.EnemiesNum` _returnvalue)
    (if (== _returnvalue 0)
      (`self.StartNewWave`))))

(event `ResetGame`
  (bind _output_classtospawn (break `/Game/Blueprints/WaveStruct` (`|GetArrayItem` (`self.Waves`) (`self.WaveIndex`))))
  (set `self.WaveIndex` 0)
  (bind _output_get (set `self.Queue` _output_classtospawn :!label _label))
  (`KismetArrayLibrary.Array_Shuffle` _output_get))

(event `StartNewWave`
  ;[1 1 1] Wave Initialization
  (`/Engine/EditorBlueprintResources/StandardMacros.IncrementInt` (`self.WaveIndex`)
    (:`  `
      (`self.NewWave`)
      (if (< (`KismetArrayLibrary.Array_LastIndex` (`self.Waves`)) (`self.WaveIndex`))
        (`self.EndGame`)
        (else
          (goto _label))))))

(event `EndGame`
  ;[1 1 1] EndGame
  (`self.EndGameDispatcher`)
  (bind _outactors (`GameplayStatics.GetAllActorsOfClass` "/Script/Engine.CameraActor"))
  (`PlayerController.SetViewTargetWithBlend` (`GameplayStatics.GetPlayerController` 0) (`|GetArrayItem` _outactors (`KismetMathLibrary.RandomInteger` (`KismetArrayLibrary.Array_Length` _outactors))) 4.0 "VTBlend_Linear" 0.0 true)
  (`KismetSystemLibrary.Delay` 5.0)
  (`GameplayStatics.OpenLevel` "MainMenu"))

(fn `SpawnDefaultPawnFor`
  (params (NewPlayer :type "Controller Object Reference") (StartSpot :type "Actor Object Reference"))
  (returns (ReturnValue :type "Pawn Object Reference"))
  (bind _outactors (`GameplayStatics.GetAllActorsOfClass` "/Game/Blueprints/ControledPlayerStart.ControledPlayerStart_C"))
  (bind _returnvalue (`|SpawnActorFromClass` (`/Game/Blueprints/KnightGameInstance.DefaultPawnClass` (cast `/Game/Blueprints/KnightGameInstance` (`GameplayStatics.GetGameInstance`) :!pure true)) (`SceneComponent.K2_GetComponentToWorld` (`/Game/Blueprints/ControledPlayerStart.DefaultSceneRoot` (`|GetArrayItem` _outactors))) "Undefined" "OverrideRootScale" NewPlayer null))
  (return _returnvalue))

(fn `UserConstructionScript`)