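; Knight war shout aura actor, attached to a character, that damages nearby characters for as long as that character's player has mana.
; A looping half-second timer drains ManaCost from the instigating player controller, then sphere-overlaps around WarrSparks and damages every KGCharacterBase found except the owner, with no team check.
; When mana is insufficient, it clears the owner's Shield flag and destroys itself.
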(event `self.ReceiveBeginPlay`
  (`KismetSystemLibrary.K2_SetTimerDelegate` (delegate `TryDealDamage`) 0.5 true))

(event `TryDealDamage`
  (bind _manacost (`self.ManaCost`))
  (bind _returnvalue (`ActorComponent.GetOwner` (`SceneComponent.GetAttachParent` (`self.DefaultSceneRoot`))))
  (bind _askc_player_controler_base (cast `/Game/Blueprints/KC_PlayerControlerBase` (`self.GetInstigatorController` _returnvalue)))
  (bind _playermana (`/Game/Blueprints/KC_PlayerControlerBase.PlayerMana` _askc_player_controler_base))
  (if (> _playermana _manacost)
    (set `/Game/Blueprints/KC_PlayerControlerBase.PlayerMana` (- _playermana _manacost) _askc_player_controler_base)
    (bind _outactors (`KismetSystemLibrary.SphereOverlapActors` (`SceneComponent.K2_GetComponentLocation` (`self.WarrSparks`)) 120.0 (`|MakeArray` "ObjectTypeQuery3" :!type "EObjectTypeQuery Enum") "/Game/Blueprints/KGCharacterBase.KGCharacterBase_C" (`|MakeArray` (`ActorComponent.GetOwner` (`SceneComponent.GetAttachParent` (`self.DefaultSceneRoot`))))))
    (for _array_element _outactors
      (`GameplayStatics.ApplyDamage` _array_element 10.0))
    (else
      (set `/Game/Blueprints/KGCharacterBase.Shield` false (cast `/Game/Blueprints/KGCharacterBase` _returnvalue :!pure true))
      (`self.K2_DestroyActor`))))

(fn `UserConstructionScript`)