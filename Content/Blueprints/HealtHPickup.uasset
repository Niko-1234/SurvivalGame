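; Health pickup actor that heals a KGCharacterBase that overlaps it and is not already at full health.
; On overlap it adds HealthOffering to Health, capped at MaxHealth, refreshes the character's health circle, then destroys itself.
; A positive sound plays at the Sphere's location only when the character is controlled by a KC_PlayerControlerBase.
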(event `self.ReceiveActorBeginOverlap`
  (params (OtherActor :type "Actor Object Reference"))
  (bind _askgcharacter_base (cast `/Game/Blueprints/KGCharacterBase` OtherActor))
  (bind _maxhealth (`/Game/Blueprints/KGCharacterBase.MaxHealth` _askgcharacter_base))
  (if (not (== (`/Game/Blueprints/KGCharacterBase.Health` _askgcharacter_base) _maxhealth))
    (set `/Game/Blueprints/KGCharacterBase.Health` (`KismetMathLibrary.FMin` _maxhealth (+ (`/Game/Blueprints/KGCharacterBase.Health` _askgcharacter_base) (`self.HealthOffering`))) _askgcharacter_base)
    (`/Game/Blueprints/KGCharacterBase.SetHealthCircle` _askgcharacter_base)
    (if (`.bSuccess` (cast `/Game/Blueprints/KC_PlayerControlerBase` (`Pawn.GetController` _askgcharacter_base) :!pure true))
      (`GameplayStatics.SpawnSoundAtLocation` "/Game/Assets/Sounds/MagicPositiveSound.MagicPositiveSound" (`SceneComponent.K2_GetComponentLocation` (`self.Sphere`)) (struct) 0.5 1.0 0.0 null null))
    (`self.K2_DestroyActor`)))

(fn `UserConstructionScript`)