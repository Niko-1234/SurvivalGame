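; Base knight character shared by player and AI, providing sword melee, magic and health.
; Attack events play montages, chaining combo sections on repeat presses; separate events spawn projectiles and a shielding war shout.
; Damage updates a material-driven health circle and triggers flinching or death, ending the game for players or randomly dropping mana for AI.
; Survivors dance on the game mode's end-game dispatcher; construction tints the tabard.
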(event `Create2HSword`
  ;[1 1 1] Create 2H Sword
  (bind _returnvalue (`|SpawnActorFromClass` "/Game/Blueprints/2HBaseSword.2HBaseSword_C" (`self.GetTransform`) "Undefined" "OverrideRootScale" null null))
  (`self.K2_AttachToComponent` _returnvalue (`self.Mesh`) "Sword" "SnapToTarget" "SnapToTarget" "SnapToTarget" false)
  (set `self.Weapon` _returnvalue))

(event `CreateSword`
  ;[1 1 1] CreateSword
  (bind _returnvalue (`|SpawnActorFromClass` "/Game/Blueprints/BaseSword.BaseSword_C" (`self.GetTransform`) "Undefined" "OverrideRootScale" null null))
  (`self.K2_AttachToComponent` _returnvalue (`self.Mesh`) "Sword" "SnapToTarget" "SnapToTarget" "SnapToTarget" false)
  (set `self.Weapon` _returnvalue))

(event `self.ReceiveTick`
  (params (DeltaSeconds :type "Float (single-precision)"))
  (`AudioComponent.SetVolumeMultiplier` (`self.KnightStepSound`) (`KismetMathLibrary.FClamp` (/ (`KismetMathLibrary.VSize` (`self.GetVelocity`)) 1000.0) 0.0 0.8)))

(event `self.ReceiveBeginPlay`
  (`self.CreateWeapon`)
  (set `self.MaxHealth` (`self.Health`))
  (`self.SetHealthCircle`)
  (bind _asknight_game_mode (cast `/Game/Blueprints/KnightGameMode` (`GameplayStatics.GetGameMode`)))
  (add `/Game/Blueprints/KnightGameMode.EndGameDispatcher` _asknight_game_mode (delegate `EndGameDance`)))

(event `EndGameDance`
  ;[1 1 1] EndGame
  (if (> (`self.Health`) 0.0)
    (`CharacterMovementComponent.DisableMovement` (`self.CharacterMovement`))
    (`self.PlayAnimMontage` "/Game/Assets/Knight/VictoryDance.VictoryDance")))

(event `CreateWeapon`
  ;[1 1 1] Default weapon and spell
  (`self.CreateSword`))

(event `TryMagic`
  ;[1 1 1] Default weapon and spell
  (`self.MagicShoot`))

(event `TryMelee`
  ;[1 1 1] Default weapon and spell
  (`self.Try1HMelee`))

(event `UsePrimaryAttack`
  ;[1 1 1] Primary attack of knight enemy
  (`self.Try1HMelee`))

(event `self.ReceiveAnyDamage`
  (params (Damage :type "Float (single-precision)") (DamageType :type "DamageType Object Reference") (InstigatedBy :type "Controller Object Reference") (DamageCauser :type "Actor Object Reference"))
  (bind _returnvalue (`SkeletalMeshComponent.GetAnimInstance` (`self.Mesh`)))
  (if (not (`self.Shield`))
    ;[1 1 1] Get Any Damage
    (bind _output_get (set `self.Health` (- (`self.Health`) Damage)))
    (`self.SetHealthCircle`)
    ;[1 1 1] Dying
    (if (<= _output_get 0.0)
      (`/Engine/EditorBlueprintResources/StandardMacros.DoOnce` false
        (:`Completed`
          (set `self.IsFlinching` true)
          (`CharacterMovementComponent.DisableMovement` (`self.CharacterMovement`))
          (if (`Controller.IsPlayerController` (`self.GetController`))
            ;[1 1 1] Player death
            (`self.PlayAnimMontage` "/Game/Assets/Knight/PlayerDeath.PlayerDeath")
            (`KismetSystemLibrary.Delay` 2.5)
            (`self.PlayerDeath`)
            (`/Game/Blueprints/KnightGameMode.EndGame` (cast `/Game/Blueprints/KnightGameMode` (`GameplayStatics.GetGameMode`) :!pure true))
            (else
              (`self.DetachFromControllerPendingDestroy`)
              (`self.PlayAnimMontage` "/Game/Assets/Knight/PlayerDeath.PlayerDeath")
              (`KismetSystemLibrary.Delay` 2.5)
              ;[1 1 1] AI DEath
              (if (== (`KismetMathLibrary.RandomInteger` 2) 0)
                (`|SpawnActorFromClass` "/Game/Blueprints/ManaPickup.ManaPickup_C" (`self.GetTransform`) "Undefined" "OverrideRootScale" null null))
              (`self.K2_DestroyActor` (`self.Weapon`))
              (`self.K2_DestroyActor`)))))
      (else
        ;[1 1 1] Flinching
        (set `self.IsFlinching` true)
        (if (`AnimInstance.Montage_IsActive` _returnvalue "/Game/Assets/Knight/KnightAttackMontage.KnightAttackMontage")
          (if (`KismetArrayLibrary.Array_Contains` (`self.AttackMoves`) (`AnimInstance.Montage_GetCurrentSection` _returnvalue "/Game/Assets/Knight/KnightAttackMontage.KnightAttackMontage"))
            (set `self.IsFlinching` false)
            (else
              (bind _returnvalue_2 (`self.PlayAnimMontage` "/Game/Assets/Knight/PlayerFlinch.PlayerFlinch" 1.0 "FlinchBig"))
              (`KismetSystemLibrary.Delay` _returnvalue_2)
              (set `self.IsFlinching` false)))
          (else
            (bind _returnvalue_3 (`self.PlayAnimMontage` "/Game/Assets/Knight/PlayerFlinch.PlayerFlinch" 1.0 "FlinchSmall"))
            (`KismetSystemLibrary.Delay` _returnvalue_3)
            (set `self.IsFlinching` false)))))))

(event `MagicShoot`
  ;[1 1 1] Do this after right click
  (if (not (`self.IsFlinching`))
    (`self.PlayAnimMontage` "/Game/Assets/Knight/MagicShootMontage.MagicShootMontage")))

(event `WarrShout`
  ;[1 1 1] Magic Warr Shout
  (if (not (or (`self.IsFlinching`) (`self.Shield`)))
    (set `self.Shield` true)
    (`GameplayStatics.SpawnSoundAttached` "/Game/Assets/Sounds/Scream.Scream" (`self.Mesh`) "None" (0.0 0.0 0.0) (struct) "KeepRelativeOffset" false 1.0 0.6 0.0 null null)
    (`self.PlayAnimMontage` "/Game/Assets/Knight/WarrShout.WarrShout")
    (bind _returnvalue (`|SpawnActorFromClass` "/Game/Blueprints/KnightWarrShout.KnightWarrShout_C" (`self.GetTransform`) "Undefined" "OverrideRootScale" null null))
    (`self.K2_AttachToComponent` _returnvalue (`self.Mesh`) "BaseSocket" "SnapToTarget" "SnapToTarget" "SnapToTarget" true)))

(event `LaunchMagicProjectile`
  ;[1 1 1] Create Actor "Knight Project Base" which deal damage
  (`|SpawnActorFromClass` "/Game/Blueprints/KnightProjectBase.KnightProjectBase_C" (`SceneComponent.K2_GetComponentToWorld` (`self.Arrow1`)) "Undefined" "OverrideRootScale" null self))

(event `Try1HMelee`
  (bind _returnvalue (`SkeletalMeshComponent.GetAnimInstance` (`self.Mesh`)))
  (bind _returnvalue_2 (`AnimInstance.Montage_GetCurrentSection` _returnvalue "/Game/Assets/Knight/KnightAttackMontage.KnightAttackMontage"))
  ;[1 1 1] Try Meele
  (if (`self.IsFlinching`)
    _
    (elif (`AnimInstance.Montage_IsActive` _returnvalue "/Game/Assets/Knight/KnightAttackMontage.KnightAttackMontage")
      (switch `name` _returnvalue_2
        (:`Attack1`
          (`AnimInstance.Montage_SetNextSection` _returnvalue _returnvalue_2 "Attack2" "/Game/Assets/Knight/KnightAttackMontage.KnightAttackMontage")))
      (else
        (`self.PlayAnimMontage` "/Game/Assets/Knight/KnightAttackMontage.KnightAttackMontage" 1.0 "Attack1")))))

(event `SetHealthCircle`
  ;[1 1 1] Circle health
  (bind _returnvalue (`PrimitiveComponent.CreateDynamicMaterialInstance` (`self.Plane`) 0 null "None"))
  (`MaterialInstanceDynamic.SetVectorParameterValue` _returnvalue "Colour" (`self.HealthBarColor`))
  (`MaterialInstanceDynamic.SetScalarParameterValue` _returnvalue "Decimal" (/ (`self.Health`) (`self.MaxHealth`))))

(event `Try2HMelee`
  (bind _returnvalue (`SkeletalMeshComponent.GetAnimInstance` (`self.Mesh`)))
  (bind _returnvalue_2 (`AnimInstance.Montage_GetCurrentSection` _returnvalue "/Game/Assets/Knight/Knight2HAttackMontage.Knight2HAttackMontage"))
  ;[1 1 1] Try2HMeele
  (if (`self.IsFlinching`)
    _
    (elif (`AnimInstance.Montage_IsActive` _returnvalue "/Game/Assets/Knight/Knight2HAttackMontage.Knight2HAttackMontage")
      (switch `name` _returnvalue_2
        (:`2HAttack1`
          (`AnimInstance.Montage_SetNextSection` _returnvalue _returnvalue_2 "2HAttack2" "/Game/Assets/Knight/Knight2HAttackMontage.Knight2HAttackMontage")))
      (else
        (`self.PlayAnimMontage` "/Game/Assets/Knight/Knight2HAttackMontage.Knight2HAttackMontage" 1.0 "2HAttack1")))))

(fn `UserConstructionScript`
  (bind _returnvalue (`PrimitiveComponent.CreateDynamicMaterialInstance` (`self.Mesh`) 0 null "None"))
  (`MaterialInstanceDynamic.SetVectorParameterValue` _returnvalue "TabardColor" (`self.TabardColor`)))