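; Base projectile actor for the Knight that damages characters it hits and explodes when destroyed.
; On overlap with a KGCharacterBase other than its instigator, it applies damage credited to the instigator's controller and destroys itself.
; The Destroyed event plays the explosion sound and impact particles and applies small radial damage, so this blast follows any destruction, not only hits.
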(event `self.ReceiveActorBeginOverlap`
  (params (OtherActor :type "Actor Object Reference"))
  (bind _instigator (`self.Instigator`))
  ;[1 1 1] Deal damage when hit an actor
  (bind _askgcharacter_base (cast `/Game/Blueprints/KGCharacterBase` OtherActor))
  (if (not (== _askgcharacter_base _instigator))
    (`GameplayStatics.ApplyDamage` _askgcharacter_base 50.0 (`Pawn.GetController` _instigator) self)
    (`self.K2_DestroyActor`)))

(event `self.ReceiveDestroyed`
  ;[1 1 1] What happen if actor is destorying
  (`GameplayStatics.SpawnSoundAttached` "/Game/Assets/Sounds/ExplosionSound.ExplosionSound" (`self.FlightSystem`) "None" (0.0 0.0 0.0) (struct) "KeepRelativeOffset" false 0.4 1.0 0.0 null null)
  (`GameplayStatics.SpawnEmitterAtLocation` "/Game/Assets/Effects/P_Impulse.P_Impulse" (`self.K2_GetActorLocation`))
  (`GameplayStatics.ApplyRadialDamage` :`BaseDamage` 20.0 :`Origin` (`self.K2_GetActorLocation`) :`DamageRadius` 50.0 :`DamageCauser` self :`InstigatedByController` (`Pawn.GetController` (`self.Instigator`))))

(fn `UserConstructionScript`)