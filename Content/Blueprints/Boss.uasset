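; Boss enemy Blueprint, a knight that wields a two-handed sword and drives a dedicated boss health bar on the player HUD.
; It overrides parent events to create the sword and attempt a one-handed melee as its primary attack.
; Health updates feed both a dynamic material on its health circle plane and the HUD bar, which is shown on BeginPlay.
; Each tick, movement speed scales the knight footstep sound's volume.
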(event `self.ReceiveBeginPlay`
  (`parent.ReceiveBeginPlay`)
  (bind _askc_player_controler_base (cast `/Game/Blueprints/KC_PlayerControlerBase` (`GameplayStatics.GetPlayerController` 0)))
  (`Widget.SetVisibility` (`/Game/Blueprints/UIHUD.BossHealthBar` (`/Game/Blueprints/KC_PlayerControlerBase.WidgetHUD` _askc_player_controler_base)) "Visible"))

(event `self.ReceiveTick`
  (params (DeltaSeconds :type "Float (single-precision)"))
  (`AudioComponent.SetVolumeMultiplier` (`self.KnightStepSound`) (`KismetMathLibrary.FClamp` (/ (`KismetMathLibrary.VSize` (`self.GetVelocity`)) 500.0) 0.0 1.5)))

(event `self.CreateWeapon`
  (`self.Create2HSword`))

(event `self.UsePrimaryAttack`
  (`self.Try1HMelee`))

(event `self.SetHealthCircle`
  (bind _returnvalue (/ (`self.Health`) (`self.MaxHealth`)))
  (bind _returnvalue_2 (`PrimitiveComponent.CreateDynamicMaterialInstance` (`self.Plane`) 0 null "None"))
  (`MaterialInstanceDynamic.SetVectorParameterValue` _returnvalue_2 "Colour" (`self.HealthBarColor`))
  (`MaterialInstanceDynamic.SetScalarParameterValue` _returnvalue_2 "Decimal" _returnvalue)
  (bind _askc_player_controler_base (cast `/Game/Blueprints/KC_PlayerControlerBase` (`GameplayStatics.GetPlayerController` 0)))
  (`ProgressBar.SetPercent` (`/Game/Blueprints/UIHUD.BossHealthBar` (`/Game/Blueprints/KC_PlayerControlerBase.WidgetHUD` _askc_player_controler_base)) _returnvalue))

(fn `UserConstructionScript`
  (`parent.UserConstructionScript`))