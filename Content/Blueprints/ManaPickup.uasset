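; Mana pickup actor that restores mana to a player who overlaps it.
; On overlap it casts the actor to KGCharacterBase and its controller to KC_PlayerControlerBase, where mana is stored.
; If mana is not full, it adds ManaOffering clamped to the maximum, plays a positive sound at the sphere and destroys itself; otherwise it stays in place.
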(event `self.ReceiveActorBeginOverlap`
  (params (OtherActor :type "Actor Object Reference"))
  (bind _askgcharacter_base (cast `/Game/Blueprints/KGCharacterBase` OtherActor))
  (bind _askc_player_controler_base (cast `/Game/Blueprints/KC_PlayerControlerBase` (`Pawn.GetController` _askgcharacter_base)))
  (bind _playermaxmana (`/Game/Blueprints/KC_PlayerControlerBase.PlayerMaxMana` _askc_player_controler_base))
  (if (not (== (`/Game/Blueprints/KC_PlayerControlerBase.PlayerMana` _askc_player_controler_base) _playermaxmana))
    (set `/Game/Blueprints/KC_PlayerControlerBase.PlayerMana` (`KismetMathLibrary.FMin` _playermaxmana (+ (`/Game/Blueprints/KC_PlayerControlerBase.PlayerMana` _askc_player_controler_base) (`self.ManaOffering`))) _askc_player_controler_base)
    (`GameplayStatics.SpawnSoundAtLocation` "/Game/Assets/Sounds/MagicPositiveSound.MagicPositiveSound" (`SceneComponent.K2_GetComponentLocation` (`self.Sphere`)) (struct) 0.5 1.0 0.0 null null)
    (`self.K2_DestroyActor`)))

(fn `UserConstructionScript`)