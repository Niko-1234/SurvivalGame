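; Base player controller for a wave-based knight game, handling cursor aiming, camera-relative movement, jump, attacks and pause.
; BeginPlay creates the HUD and binds game mode wave and character death events to text animations.
; Tick turns the living pawn toward the cursor hit while waves remain and refreshes health and mana bars.
; The controller owns mana, deducting spell cost after a delay or playing a throttled no-mana voice line.
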(event `SetManaBar`
  ;[1 1 1] Set mana bar
  (`ProgressBar.SetPercent` (`/Game/Blueprints/UIHUD.PlayerManaBar` (`self.WidgetHUD`)) (/ (`self.PlayerMana`) (`self.PlayerMaxMana`))))

(event `SetHealthBar`
  (bind _askgcharacter_base (cast `/Game/Blueprints/KGCharacterBase` (`self.K2_GetPawn`) :!pure true))
  ;[1 1 1] Set health bar
  (`ProgressBar.SetPercent` (`/Game/Blueprints/UIHUD.PlayerHealthBar` (`self.WidgetHUD`)) (/ (`/Game/Blueprints/KGCharacterBase.Health` _askgcharacter_base) (`/Game/Blueprints/KGCharacterBase.MaxHealth` _askgcharacter_base))))

(event `self.ReceiveBeginPlay`
  ;[1 1 1] HUD UI
  (set `self.bShowMouseCursor` true)
  (set `self.PlayerMana` (`self.PlayerMaxMana`))
  (bind _returnvalue (`|CreateWidget` "/Game/Blueprints/UIHUD.UIHUD_C"))
  (bind _output_get (set `self.WidgetHUD` _returnvalue))
  (`UserWidget.AddToViewport` _output_get 0)
  (bind _asknight_game_mode (cast `/Game/Blueprints/KnightGameMode` (`GameplayStatics.GetGameMode`)))
  (add `/Game/Blueprints/KnightGameMode.NewWave` _asknight_game_mode (delegate `PopUpWaveText`))
  (bind _askgcharacter_base (cast `/Game/Blueprints/KGCharacterBase` (`GameplayStatics.GetPlayerCharacter` 0)))
  (add `/Game/Blueprints/KGCharacterBase.PlayerDeath` _askgcharacter_base (delegate `ShowDeathText`)))

(event `PopUpWaveText`
  (bind _widgethud (`self.WidgetHUD`))
  ;[1 1 1] HUD UI
  (`UserWidget.PlayAnimation` _widgethud (`/Game/Blueprints/UIHUD.WaveCompletedAnimUp` _widgethud) 0.0 1 "Forward" 1.0))

(event `ShowDeathText`
  (bind _widgethud (`self.WidgetHUD`))
  ;[1 1 1] HUD UI
  (`UserWidget.PlayAnimation` _widgethud (`/Game/Blueprints/UIHUD.DeathTextUp` _widgethud) 0.0 1 "Forward" 1.0))

(event `ShowPasue`
  ;[1 1 1] HUD UI
  (`Widget.SetVisibility` (stale `self.ReceiveBeginPlay` _returnvalue) "Visible")
  (`Widget.SetVisibility` (`/Game/Blueprints/UIHUD.GamePauseBox` (stale `self.ReceiveBeginPlay` _returnvalue)) "Visible"))

(event `self.ReceiveTick`
  (params (DeltaSeconds :type "Float (single-precision)"))
  (`self.ProcessMouse`)
  (`self.SetHealthBar`)
  (`self.SetManaBar`))

(event `ProcessMouse`
  (bind (_hitresult _returnvalue) (`self.GetHitResultUnderCursorByChannel` "TraceTypeQuery1"))
  (bind _returnvalue_2 (`self.K2_GetPawn`))
  (bind _returnvalue_3 (`self.K2_GetPawn`))
  (bind (_returnvalue_roll _returnvalue_pitch _returnvalue_yaw) (`KismetMathLibrary.BreakRotator` (`KismetMathLibrary.Conv_VectorToRotator` (`KismetMathLibrary.GetDirectionUnitVector` (`self.K2_GetActorLocation` _returnvalue_3) (`.Location` (`GameplayStatics.BreakHitResult` _hitresult))))))
  ;[1 1 1] Mouse proces
  (`/Engine/EditorBlueprintResources/StandardMacros.IsValid` _returnvalue_2
    (:`Is Valid`
      (bind _askgcharacter_base (cast `/Game/Blueprints/KGCharacterBase` _returnvalue_2))
      (bind _asknight_game_mode (cast `/Game/Blueprints/KnightGameMode` (`GameplayStatics.GetGameMode`)))
      (if (and (> (`/Game/Blueprints/KGCharacterBase.Health` _askgcharacter_base) 0.0) _returnvalue (>= (`KismetArrayLibrary.Array_LastIndex` (`/Game/Blueprints/KnightGameMode.Waves` _asknight_game_mode)) (`/Game/Blueprints/KnightGameMode.WaveIndex` _asknight_game_mode)) (not (`GameplayStatics.IsGamePaused`)))
        (`self.K2_SetActorRotation` _returnvalue_3 (`KismetMathLibrary.MakeRotator` 0.0 0.0 _returnvalue_yaw) false)))))

(event `InputAxis|Up`
  (params (AxisValue :type "Float (single-precision)"))
  (bind _returnvalue (`self.K2_GetPawn`))
  ;[1 1 1] movement
  (`/Engine/EditorBlueprintResources/StandardMacros.IsValid` _returnvalue
    (:`Is Valid`
      (`Pawn.AddMovementInput` _returnvalue (`SceneComponent.GetUpVector` (`PlayerCameraManager.TransformComponent` (`self.PlayerCameraManager`))) AxisValue false))))

(event `InputAxis|Right`
  (params (AxisValue :type "Float (single-precision)"))
  (bind _returnvalue (`self.K2_GetPawn`))
  ;[1 1 1] movement
  (`/Engine/EditorBlueprintResources/StandardMacros.IsValid` _returnvalue
    (:`Is Valid`
      (`Pawn.AddMovementInput` _returnvalue (`SceneComponent.GetRightVector` (`PlayerCameraManager.TransformComponent` (`self.PlayerCameraManager`))) AxisValue false))))

(event `InputAction|Jump`
  (params (Key :type "Key Structure"))
  ;[1 1 1] movement
  (:`Pressed`
    (bind _ascharacter (cast `Character` (`self.K2_GetPawn`)))
    (`Character.Jump` _ascharacter)))

(event `InputAction|MeleeAttack`
  (params (Key :type "Key Structure"))
  ;[1 1 1] attacs
  (:`Pressed`
    (bind _askgcharacter_base (cast `/Game/Blueprints/KGCharacterBase` (`self.K2_GetPawn`)))
    (`/Game/Blueprints/KGCharacterBase.TryMelee` _askgcharacter_base)))

(event `InputAction|MagicAttack`
  (params (Key :type "Key Structure"))
  (bind _playermana (`self.PlayerMana`))
  (bind _spellcost (`self.SpellCost`))
  ;[1 1 1] attacs
  (:`Pressed`
    (bind _askgcharacter_base (cast `/Game/Blueprints/KGCharacterBase` (`self.K2_GetPawn`)))
    (if (`/Game/Blueprints/KGCharacterBase.Shield` _askgcharacter_base)
      _
      (elif (>= _playermana _spellcost)
        (`/Game/Blueprints/KGCharacterBase.TryMagic` _askgcharacter_base)
        (`KismetSystemLibrary.Delay` 1.0)
        ;[1 1 1] Mana say
        (set `self.PlayerMana` (- _playermana _spellcost))
        (else
          (`self.PlayMana Dialogue`))))))

(event `PlayMana Dialogue`
  ;[1 1 1] Mana say
  (if (not (`self.IsPlaying`))
    (bind _returnvalue (`GameplayStatics.SpawnSoundAttached` "/Game/Assets/Sounds/nomanaSound.nomanaSound" (`Character.Mesh` (cast `/Game/Blueprints/KGCharacterBase` (`self.K2_GetPawn`) :!pure true)) "None" (0.0 0.0 0.0) (struct) "KeepRelativeOffset" false 0.6 1.0 0.0 null null))
    (set `self.IsPlaying` (`AudioComponent.IsPlaying` _returnvalue))
    (`KismetSystemLibrary.Delay` 1.7)
    (set `self.IsPlaying` false)))

(event `InputAction|Pause`
  (params (Key :type "Key Structure"))
  ;[1 1 1] pause
  (:`Pressed`
    (if (not (`GameplayStatics.IsGamePaused`))
      (`GameplayStatics.SetGamePaused` true)
      (`self.ShowPasue`))))

(fn `UserConstructionScript`)